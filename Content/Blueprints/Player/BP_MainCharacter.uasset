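; Main player character Blueprint that decides when a stealth level is won or lost.
; Every Tick it counts dead BP_GuardEnemy actors; all down shows the win screen on Urban_Map or game-ended screen elsewhere, skipping MainMenu.
; Otherwise, HasBeenSeen triggers defeat then lose screens, while HasBeenHeard clears after a delay.
; End states disable input, hide the crosshair and pause after a delay, re-creating their first widget each Tick until then.
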(event `self.ReceiveBeginPlay`)

(event `self.ReceiveActorBeginOverlap`
  (params (OtherActor :type "Actor Object Reference")))

(event `self.ReceiveTick`
  (params (DeltaSeconds :type "Float (single-precision)"))
  (bind _areallenemiesdown (`self.AreAllEnemiesDown`))
  (if _areallenemiesdown
    (bind _returnvalue (`GameplayStatics.GetCurrentLevelName` true))
    (if (`KismetStringLibrary.EqualEqual_StrStr` _returnvalue "Urban_Map")
      (`self.DisableInput` (`GameplayStatics.GetPlayerCharacter` 0) (`GameplayStatics.GetPlayerController` 0))
      (bind _returnvalue_2 (`|CreateWidget` "/Game/UI/WBG_WinScreen.WBG_WinScreen_C"))
      (`UserWidget.AddToViewport` _returnvalue_2 0)
      (bind _foundwidgets (`WidgetBlueprintLibrary.GetAllWidgetsOfClass` "/Game/UI/WBP_Crosshair.WBP_Crosshair_C"))
      (`Widget.SetVisibility` _foundwidgets "Hidden")
      (`KismetSystemLibrary.Delay` 1.0)
      (set `PlayerController.bShowMouseCursor` true (`GameplayStatics.GetPlayerController` 0))
      (`GameplayStatics.SetGamePaused` true)
      (elif (not (`KismetStringLibrary.EqualEqual_StrStr` _returnvalue "MainMenu"))
        (`self.DisableInput` (`GameplayStatics.GetPlayerCharacter` 0) (`GameplayStatics.GetPlayerController` 0))
        (bind _returnvalue_3 (`|CreateWidget` "/Game/UI/WBG_GameEnded.WBG_GameEnded_C"))
        (`UserWidget.AddToViewport` _returnvalue_3 0)
        (bind _foundwidgets_2 (`WidgetBlueprintLibrary.GetAllWidgetsOfClass` "/Game/UI/WBP_Crosshair.WBP_Crosshair_C"))
        (`Widget.SetVisibility` _foundwidgets_2 "Hidden")
        (`KismetSystemLibrary.Delay` 1.0)
        (set `PlayerController.bShowMouseCursor` true (`GameplayStatics.GetPlayerController` 0))
        (`GameplayStatics.SetGamePaused` true)))
    (elif (`self.HasBeenSeen`)
      (`self.DisableInput` (`GameplayStatics.GetPlayerCharacter` 0) (`GameplayStatics.GetPlayerController` 0))
      (bind _returnvalue_4 (`|CreateWidget` "/Game/UI/WBG_Defeat.WBG_Defeat_C"))
      (`UserWidget.AddToViewport` _returnvalue_4 0)
      (bind _foundwidgets_3 (`WidgetBlueprintLibrary.GetAllWidgetsOfClass` "/Game/UI/WBP_Crosshair.WBP_Crosshair_C"))
      (`Widget.SetVisibility` _foundwidgets_3 "Hidden")
      (`KismetSystemLibrary.Delay` 3.0)
      (bind _returnvalue_5 (`|CreateWidget` "/Game/UI/WBG_LoseScreen.WBG_LoseScreen_C"))
      (`UserWidget.AddToViewport` _returnvalue_5 0)
      (set `PlayerController.bShowMouseCursor` true (`GameplayStatics.GetPlayerController` 0))
      (`GameplayStatics.SetGamePaused` true)
      (elif (`self.HasBeenHeard`)
        (`KismetSystemLibrary.Delay` 3.0)
        (set `self.HasBeenHeard` false)))))

(fn `AreAllEnemiesDown`
  (returns (AreAllEnemiesDown :type Boolean))
  (locals (HowManyDown :type Integer))
  (set `local.HowManyDown` 0)
  (bind _outactors (`GameplayStatics.GetAllActorsOfClass` "/Game/Blueprints/AI/BP_GuardEnemy.BP_GuardEnemy_C"))
  (for _array_element _outactors
    (bind _asbp_guard_enemy (cast `/Game/Blueprints/AI/BP_GuardEnemy` _array_element))
    (if (`self.IsDead` _asbp_guard_enemy)
      (set `local.HowManyDown` (+ (`local.HowManyDown`) 1))))
  (return (== (`KismetArrayLibrary.Array_Length` _outactors) (`local.HowManyDown`))))

(fn `UserConstructionScript`)